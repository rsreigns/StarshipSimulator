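; Base Blueprint for enemy ships that grants a missile ability and manages an on-screen health widget.
; On BeginPlay it gives GAMissile to its ability system component and adds a collapsed enemy health widget to the viewport.
; ShowWidget reveals the widget and restarts a timer that hides it again after a few seconds.
; UpdateHealthUI forwards health percent, current and max values to the widget.
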(event `self.ReceiveBeginPlay`
  (`AbilitySystemComponent.K2_GiveAbility` (`self.BaseASC`) "/Game/MyFiles/Gameplay/Abilities/Player/GAMissile.GAMissile_C" 1 -1)
  (bind _returnvalue (`|CreateWidget` "/Game/MyFiles/UI/WBP_EnemyHealthWidget.WBP_EnemyHealthWidget_C" (`GameplayStatics.GetPlayerController` 0)))
  (set `self.healthUI` _returnvalue)
  (`UserWidget.AddToViewport` _returnvalue 0)
  (`Widget.SetVisibility` (`self.healthUI`) "Collapsed"))

(event `self.ReceiveTick`
  (params (DeltaSeconds :type "Float (single-precision)")))

(event `self.ShowWidget`
  (if (`KismetSystemLibrary.K2_IsTimerActiveHandle` (`self.HideTimer`))
    (`KismetSystemLibrary.K2_ClearAndInvalidateTimerHandle` (`self.HideTimer`)))
  (bind _returnvalue (`KismetSystemLibrary.K2_SetTimerDelegate` (delegate `HideWidget`) 4.0))
  (set `self.HideTimer` _returnvalue)
  (`Widget.SetVisibility` (`self.healthUI`) "SelfHitTestInvisible"))

(event `HideWidget`
  (`Widget.SetVisibility` (`self.healthUI`) "Collapsed"))

(event `self.UpdateHealthUI`
  (params (NewHealthPercent :type "Float (single-precision)") (CurrentHealth :type "Float (single-precision)") (MaxHealth :type "Float (single-precision)"))
  (`/Game/MyFiles/UI/WBP_EnemyHealthWidget.UpdateHealthPercent` (`self.healthUI`) NewHealthPercent CurrentHealth MaxHealth))

(fn `UserConstructionScript`)